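; Fire area actor for the Aura spreading fire ability that plays an explosion and then grows a burning zone.
; On BeginPlay it spawns a scaled fire explosion Niagara system, activates six further fire effects one by one at SpreadTime intervals, then destroys itself after a short hold.
; A box component's begin and end overlaps are forwarded to OnOverlap and OnEndOverlap, which are not defined in this graph.
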(event `self.ReceiveBeginPlay`
  (bind _spreadtime (`self.SpreadTime`))
  (`NiagaraFunctionLibrary.SpawnSystemAtLocation` "/Game/Assets/Effects/Projectiles/FireExplosion/NS_FireExplosion.NS_FireExplosion" (`SceneComponent.K2_GetComponentLocation` (`self.FireEffect`)) (struct) (2.0 2.0 2.0))
  (`KismetSystemLibrary.Delay` _spreadtime)
  (`ActorComponent.SetActive` (`self.FireEffect1`) true false)
  (`KismetSystemLibrary.Delay` _spreadtime)
  (`ActorComponent.SetActive` (`self.FireEffect2`) true false)
  (`KismetSystemLibrary.Delay` _spreadtime)
  (`ActorComponent.SetActive` (`self.FireEffect3`) true false)
  (`KismetSystemLibrary.Delay` _spreadtime)
  (`ActorComponent.SetActive` (`self.FireEffect4`) true false)
  (`KismetSystemLibrary.Delay` _spreadtime)
  (`ActorComponent.SetActive` (`self.FireEffect5`) true false)
  (`KismetSystemLibrary.Delay` _spreadtime)
  (`ActorComponent.SetActive` (`self.FireEffect6`) true false)
  (`KismetSystemLibrary.Delay` 5.0)
  (`self.K2_DestroyActor`))

(event `self.Box.OnComponentBeginOverlap`
  (params (OverlappedComponent :type "PrimitiveComponent Object Reference") (OtherActor :type "Actor Object Reference") (OtherComp :type "PrimitiveComponent Object Reference") (OtherBodyIndex :type Integer) (bFromSweep :type Boolean) (SweepResult :type "HitResult Structure (by ref)"))
  (`self.OnOverlap` OtherActor))

(event `self.Box.OnComponentEndOverlap`
  (params (OverlappedComponent :type "PrimitiveComponent Object Reference") (OtherActor :type "Actor Object Reference") (OtherComp :type "PrimitiveComponent Object Reference") (OtherBodyIndex :type Integer))
  (`self.OnEndOverlap` OtherActor))

(fn `UserConstructionScript`)