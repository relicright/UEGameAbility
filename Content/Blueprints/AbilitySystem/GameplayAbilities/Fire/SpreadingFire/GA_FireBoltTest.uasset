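; Test fire bolt gameplay ability that spawns a spreading fire area where the caster targets under the mouse.
; On valid target data, it turns the avatar toward that point, plays the fire bolt cast montage and waits for its montage gameplay event.
; The event spawns BP_FireAreaSpread at the target, yawed along the cast direction with the avatar as owner and instigator, then the ability ends after a short delay.
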(event `self.K2_ActivateAbility`
  (bind _returnvalue (`self.GetAvatarActorFromActorInfo`))
  (bind _projectiletargetlocation (`self.ProjectileTargetLocation`))
  (bind (_returnvalue_roll _returnvalue_pitch _returnvalue_yaw) (`KismetMathLibrary.BreakRotator` (`KismetMathLibrary.Conv_VectorToRotator` (- _projectiletargetlocation (`Actor.K2_GetActorLocation` _returnvalue)))))
  (bind (_asynctaskproxy _datahandle) (`TargetDataUnderMouse.CreateTargetDataUnderMouse`)
    (:`validData`
      (set `self.ProjectileTargetLocation` (`.Location` (`GameplayStatics.BreakHitResult` (`AbilitySystemBlueprintLibrary.GetHitResultFromTargetData` _datahandle))))
      (bind _ascombat_interface (cast `CombatInterface` _returnvalue))
      (`CombatInterface.UpdateFacingTarget` _ascombat_interface (`self.ProjectileTargetLocation`))
      (`AbilityTask_PlayMontageAndWait.CreatePlayMontageAndWaitProxy` "None" "/Game/Assets/Characters/Aura/Animations/Abilities/AM_Cast_FireBolt.AM_Cast_FireBolt"
        (:`then`
          (`AbilityTask_WaitGameplayEvent.WaitGameplayEvent` (struct :`TagName` "Event.Montage.FireBolt") null
            (:`EventReceived`
              (bind _aspawn (cast `Pawn` _returnvalue))
              (`|SpawnActorFromClass` "/Game/Blueprints/AbilitySystem/GameplayAbilities/Fire/SpreadingFire/BP_FireAreaSpread.BP_FireAreaSpread_C" (`KismetMathLibrary.MakeTransform` _projectiletargetlocation (`KismetMathLibrary.MakeRotator` 0.0 0.0 _returnvalue_yaw)) "Undefined" "MultiplyWithRoot" _returnvalue _aspawn)
              (`KismetSystemLibrary.Delay` 0.5)
              (`self.K2_EndAbility`))))))))